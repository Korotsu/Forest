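; Shiny eye actor that renders a pair of glowing-style eye sprites which turn relative to the player camera.
; Construction creates a dynamic instance of M_shinyEye, shared by both material billboards.
; Tick rotates the scene root from the camera direction masked by LockAxis, with pitch/roll swapped and yaw offset.
; It also reapplies eye spacing (Glabella), sprite size, intensity and day/night colors every frame.
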(event `self.ReceiveTick`
  (params (DeltaSeconds :type "Float (single-precision)"))
  (bind _scene (`self.Scene`))
  ;[1 1 1] UpdateRotation
  (`SceneComponent.K2_SetRelativeRotation` _scene (`KismetMathLibrary.MakeRotator` (.pitch (`KismetMathLibrary.Conv_VectorToRotator` (* (- (`SceneComponent.K2_GetComponentLocation` _scene) (.location (`self.GetTransform` (`GameplayStatics.GetPlayerCameraManager` 0)))) (`self.LockAxis`)))) (.roll (`KismetMathLibrary.Conv_VectorToRotator` (* (- (`SceneComponent.K2_GetComponentLocation` _scene) (.location (`self.GetTransform` (`GameplayStatics.GetPlayerCameraManager` 0)))) (`self.LockAxis`)))) (+ (.yaw (`KismetMathLibrary.Conv_VectorToRotator` (* (- (`SceneComponent.K2_GetComponentLocation` _scene) (.location (`self.GetTransform` (`GameplayStatics.GetPlayerCameraManager` 0)))) (`self.LockAxis`)))) 90.0)) false false)
  (`self.UpdateMaterial`))

(fn `ApplyGlabella`
  (params (target :type "SceneComponent Object Reference"))
  (bind _x (.x (.location (`SceneComponent.GetRelativeTransform` target))))
  (`SceneComponent.K2_SetRelativeTransform` target (`KismetMathLibrary.MakeTransform` (`KismetMathLibrary.MakeVector` (* (/ _x (`KismetMathLibrary.Abs` _x)) (`self.Glabella`))) (.rotation (`SceneComponent.GetRelativeTransform` target)) (.scale (`SceneComponent.GetRelativeTransform` target))) false false))

(fn `UpdateMaterial`
  (bind _eyesize (`self.EyeSize`))
  (bind _array (`|MakeArray` (make `MaterialSpriteElement` (`self.DynamicMaterial`) null false _eyesize _eyesize)))
  ;[1 1 1] UpdateMaterial
  (`self.ApplyGlabella` (`self.RightEye`))
  (`self.ApplyGlabella` (`self.LeftEye`))
  (`MaterialBillboardComponent.SetElements` (`self.LeftEye`) _array)
  (`MaterialBillboardComponent.SetElements` (`self.RightEye`) _array)
  (`MaterialInstanceDynamic.SetScalarParameterValue` (`self.DynamicMaterial`) "Intensity" (`self.Intensity`))
  (`MaterialInstanceDynamic.SetVectorParameterValue` (`self.DynamicMaterial`) "DayColor" (`self.DayColor`))
  (`MaterialInstanceDynamic.SetVectorParameterValue` (`self.DynamicMaterial`) "NightColor" (`self.NightColor`)))

(fn `UserConstructionScript`
  (locals (NewLocalVar_0 :type "MaterialBillboardComponent Object Reference"))
  (bind _returnvalue (`KismetMaterialLibrary.CreateDynamicMaterialInstance` "/Game/Materials/M/M_shinyEye.M_shinyEye"))
  (set `self.DynamicMaterial` _returnvalue)
  (`self.UpdateMaterial`))