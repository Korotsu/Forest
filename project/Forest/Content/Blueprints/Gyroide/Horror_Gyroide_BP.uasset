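; Horror gyroide actor that lurks behind the player, relocating whenever it is out of view.
; Each Tick, MoveBehindPlayer checks whether Body was rendered within TimeToVanish; if not, it moves the Scene component to BehindOffset behind the player camera along its forward vector, without sweeping.
; The construction script creates a dynamic instance of M_shinyEye and calls UpdateMaterial.
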(event `self.ReceiveTick`
  (params (DeltaSeconds :type "Float (single-precision)"))
  (`parent.ReceiveTick` DeltaSeconds)
  (`self.MoveBehindPlayer`))

(fn `MoveBehindPlayer`
  (bind _returnvalue (`GameplayStatics.GetPlayerCameraManager` 0))
  (if (not (`PrimitiveComponent.WasRecentlyRendered` (`self.Body`) (`self.TimeToVanish`)))
    (`SceneComponent.K2_SetWorldLocation` (`self.Scene`) (- (.location (`self.GetTransform` _returnvalue)) (* (`self.GetActorForwardVector` _returnvalue) (`self.BehindOffset`))) false false)))

(fn `UserConstructionScript`
  (bind _returnvalue (`KismetMaterialLibrary.CreateDynamicMaterialInstance` "/Game/Materials/M/M_shinyEye.M_shinyEye"))
  (set `self.DynamicMaterial` _returnvalue)
  (`self.UpdateMaterial`))