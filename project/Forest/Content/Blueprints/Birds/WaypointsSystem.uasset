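; Waypoint manager that flies a list of birds along a looping path of target points.
; Birds snap to the first point on construction and BeginPlay, then each Tick moves them by interpolated direction and FlockComponent speed, smoothly rotating toward their target.
; Within a stop distance, a bird advances its waypoint index, optionally teleporting to the first point on wrap-around.
; Each bird's FlockComponent tracks its index and remaining leg distance.
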(event `self.ReceiveBeginPlay`
  (`self.UpdateBirdsFirstLocation`))

(event `self.ReceiveTick`
  (params (DeltaSeconds :type "Float (single-precision)"))
  (`self.Update Birds` DeltaSeconds))

(fn `nextIndex`
  (params (prev :type Integer))
  (returns (next :type Integer))
  (return (mod (+ prev 1) (`KismetArrayLibrary.Array_Length` (`self.targetPoints`)))))

(fn `ResetToFirstWaypoint`
  (params (Bird :type "Actor Object Reference") (FlockComponent :type "/Game/Blueprints/Birds/FlockComponent Object Reference"))
  (`self.K2_SetActorLocation` Bird (`SceneComponent.K2_GetComponentLocation` (`TargetPoint.ArrowComponent` (`|GetArrayItem` (`self.targetPoints`)))) false true)
  (set `/Game/Blueprints/Birds/FlockComponent.waypointIndex` (`self.nextIndex` (`/Game/Blueprints/Birds/FlockComponent.waypointIndex` FlockComponent)) FlockComponent))

(fn `Update Birds`
  (params (deltaTime :type "Float (double-precision)"))
  (locals (targetLoc :type "Vector Structure" :default (0.0 0.0 0.0)))
  (bind _stopdistance (`self.stopDistance`))
  (for _array_element (`self.toMove`)
    (bind _flockcomponent (`/Game/Blueprints/Birds/Bird.FlockComponent` _array_element))
    (bind _waypointindex (`/Game/Blueprints/Birds/FlockComponent.waypointIndex` _flockcomponent))
    (bind _output (`|GetArrayItem` (`self.targetPoints`) _waypointindex))
    (set `local.targetLoc` (`self.K2_GetActorLocation` _output))
    (`self.UpdateBirdLocation` _array_element deltaTime (`local.targetLoc`))
    (if (< (`self.GetSquaredDistanceTo` _array_element _output) (* _stopdistance _stopdistance))
      (bind _output_get (set `/Game/Blueprints/Birds/FlockComponent.waypointIndex` (`self.nextIndex` _waypointindex) _flockcomponent))
      (`|ExecutionSequence`
        (:`then_0`
          (if (and (`self.doesTp`) (== _output_get 0))
            (set `local.targetLoc` (`self.K2_GetActorLocation` (`|GetArrayItem` (`self.targetPoints`))))
            (`self.ResetToFirstWaypoint` _array_element _flockcomponent)))
        (:`then_1`
          (set `/Game/Blueprints/Birds/FlockComponent.waypointDistanceLeft` (`KismetMathLibrary.VSize` (- (`self.K2_GetActorLocation` (`|GetArrayItem` (`self.targetPoints`) _waypointindex)) (`local.targetLoc`))) _flockcomponent))))))

(fn `UpdateBirdLocation`
  (params (bird :type "/Game/Blueprints/Birds/Bird Object Reference") (deltaTime :type "Float (double-precision)") (targetLocation :type "Vector Structure"))
  (bind _flockcomponent (`/Game/Blueprints/Birds/Bird.FlockComponent` bird))
  (bind _newvelocity (`self.UpdateBirdVelocity` bird targetLocation deltaTime))
  (bind _returnvalue (* _newvelocity (* deltaTime (`/Game/Blueprints/Birds/FlockComponent.speed` _flockcomponent))))
  (`self.K2_AddActorWorldOffset` bird _returnvalue false false)
  (set `/Game/Blueprints/Birds/FlockComponent.waypointDistanceLeft` (- (`/Game/Blueprints/Birds/FlockComponent.waypointDistanceLeft` _flockcomponent) (`KismetMathLibrary.VSize` _returnvalue)) _flockcomponent)
  (`self.K2_SetActorRotation` bird (`KismetMathLibrary.RInterpTo` (`self.K2_GetActorRotation` bird) (`KismetMathLibrary.FindLookAtRotation` (`self.K2_GetActorLocation` bird) targetLocation) deltaTime (`self.rotationInterpSpeed`)) false)
  (return))

(fn `UpdateBirdsFirstLocation`
  (bind _targetpoints (`self.targetPoints`))
  (if (`KismetArrayLibrary.Array_IsValidIndex` _targetpoints)
    (for _array_element (`self.toMove`)
      (`self.K2_SetActorLocation` _array_element (`self.K2_GetActorLocation` (`|GetArrayItem` _targetpoints)) false true))))

(fn `UpdateBirdVelocity`
  (params (bird :type "/Game/Blueprints/Birds/Bird Object Reference") (targetLocation :type "Vector Structure") (deltaTime :type "Float (double-precision)"))
  (returns (newVelocity :type "Vector Structure"))
  (bind _output_get (set `/Game/Blueprints/Birds/Bird.birdVelocity` (`KismetMathLibrary.VInterpTo` (`/Game/Blueprints/Birds/Bird.birdVelocity` bird) (`KismetMathLibrary.Normal` (- targetLocation (`self.K2_GetActorLocation` bird))) deltaTime (`self.velocityInterpSpeed`)) bird))
  (return _output_get))

(fn `UserConstructionScript`
  (`self.UpdateBirdsFirstLocation`))