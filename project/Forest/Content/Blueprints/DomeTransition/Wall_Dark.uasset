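; Wall_Dark is an actor in the DomeTransition folder that continuously spins three cylinder components.
; Each Tick it adds relative yaw to SMCylindeInt, SMCylinderExt and SMCylinderInt2, scaled by DeltaSeconds and a separate speed variable for each.
; The exterior cylinder turns with a negated speed, so it counter-rotates against the two interior ones when the speeds share a sign.
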(event `self.ReceiveTick`
  (params (DeltaSeconds :type "Float (single-precision)"))
  (`SceneComponent.K2_AddRelativeRotation` (`self.SM_Cylinde_Int`) (`KismetMathLibrary.MakeRotator` 0.0 0.0 (* DeltaSeconds (`self.Speed`))) false false)
  (`SceneComponent.K2_AddRelativeRotation` (`self.SM_Cylinder_Ext`) (`KismetMathLibrary.MakeRotator` 0.0 0.0 (* DeltaSeconds (`self.Speed_2`) -1.0)) false false)
  (`SceneComponent.K2_AddRelativeRotation` (`self.SM_Cylinder_Int_2`) (`KismetMathLibrary.MakeRotator` 0.0 0.0 (* DeltaSeconds (`self.Speed_3`) 1.0)) false false))

(fn `UserConstructionScript`)