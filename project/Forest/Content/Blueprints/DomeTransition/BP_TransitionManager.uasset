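; Manager actor that drives an expanding dome transition between day and night worlds, plus an environment swap event that skips the expansion.
; A looping timer grows Radius, feeding a material parameter collection and scaling the wall mesh, then flips isNight and resets at maximum.
; Along the way it toggles walls and particles, updates wind managers, blends the sky sphere, and switches the Gyroide's state once the radius reaches it.
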(event Custom|UpdateTransition
  ;[1 1 1] UpdateTransition
  (bind _output_get (Variables|Transition|SetRadius (+ (Variables|Transition|GetRadius) (Variables|Transition|GetTransitionSpeed))))
  (if (<= _output_get (Variables|Transition|GetRadiusMax))
    (Rendering|Material|SetScalarParameterValue "/Game/MaterialParametersCollection/TransitionParameters.TransitionParameters" "Radius" (Variables|Transition|GetRadius) :!class /Script/Engine.KismetMaterialLibrary)
    (Transformation|SetWorldScale3D (Variables|Default|GetWallScaler) (Math|Conversions|ToVector(Float) (/ (Variables|Transition|GetRadius) (Variables|Transition|GetDistanceScale))))
    (Rendering|Material|SetVectorParameterValue "/Game/MaterialParametersCollection/TransitionParameters.TransitionParameters" "Center" (Math|Conversions|ToLinearColor(Vector) (Transformation|GetActorLocation)) :!class /Script/Engine.KismetMaterialLibrary)
    (Rendering|Material|SetScalarParameterValue "/Game/MaterialParametersCollection/TransitionParameters.TransitionParameters" "Smoothness" (Variables|Transition|GetSmoothness) :!class /Script/Engine.KismetMaterialLibrary)
    (CallFunction|UpdateGyroide)
    (CallFunction|UpdateSkySphere)
    (else
      (bind _returnvalue (Rendering|Material|GetScalarParameterValue "/Game/MaterialParametersCollection/TransitionParameters.TransitionParameters" "isNight" :!class /Script/Engine.KismetMaterialLibrary))
      (Rendering|Material|SetScalarParameterValue "/Game/MaterialParametersCollection/TransitionParameters.TransitionParameters" "isNight" (* _returnvalue -1.0) :!class /Script/Engine.KismetMaterialLibrary)
      (CallFunction|ResetTransition))))

(event EventSwapEnvironmentType
  ;[1 1 1] SwapEnvironmentType
  (CallFunction|UpdateGyroide)
  (bind _returnvalue (Rendering|Material|GetScalarParameterValue "/Game/MaterialParametersCollection/TransitionParameters.TransitionParameters" "isNight" :!class /Script/Engine.KismetMaterialLibrary))
  (Rendering|Material|SetScalarParameterValue "/Game/MaterialParametersCollection/TransitionParameters.TransitionParameters" "isNight" (* _returnvalue -1.0) :!class /Script/Engine.KismetMaterialLibrary)
  (CallFunction|SwapVFX))

(event EventResetTransition
  ;[1 1 1] ResetTransition
  (bind _output_get (Variables|Transition|SetRadius 0.0))
  (CallFunction|StopTransition)
  (Rendering|Material|SetScalarParameterValue "/Game/MaterialParametersCollection/TransitionParameters.TransitionParameters" "Radius" _output_get :!class /Script/Engine.KismetMaterialLibrary)
  (Transformation|SetWorldScale3D (Variables|Default|GetWallScaler) (Math|Conversions|ToVector(Float) _output_get))
  (Rendering|Material|SetVectorParameterValue "/Game/MaterialParametersCollection/TransitionParameters.TransitionParameters" "Center" (Math|Conversions|ToLinearColor(Vector) (Transformation|GetActorLocation)) :!class /Script/Engine.KismetMaterialLibrary)
  (CallFunction|EndVFX))

(event EventStopTransition
  ;[1 1 1] StopTransition
  (Utilities|Time|PauseTimerbyHandle (Variables|Default|GetTimer)))

(event EventBeginPlay
  ;[1 1 1] BeginPlay
  (bind _outactors (Actor|GetAllActorsOfClass "/Game/Blueprints/Gyroide/Horror_Gyroide_BP.Horror_Gyroide_BP_C"))
  (bind _output_get (Variables|Gyroide|SetGyroide (Utilities|Array|Get(acopy) _outactors)))
  (Variables|Gyroide|SetInitialTransform (Transformation|GetActorTransform _output_get))
  (bind _outactors_2 (Actor|GetAllActorsOfClass "/Game/Blueprints/WindManager.WindManager_C"))
  (Variables|Default|SetWindManagerList _outactors_2)
  (bind _outactors_3 (Actor|GetAllActorsOfClass "/Game/Blueprints/SkySphere/BP_Sky_Sphere.BP_Sky_Sphere_C"))
  (Variables|Default|SetSkySphere (Utilities|Array|Get(acopy) _outactors_3))
  (bind _outactors_4 (Actor|GetAllActorsOfClass "/Game/Blueprints/BP_Bubbles.BP_Bubbles_C"))
  (Variables|Default|SetBubbleList (Utilities|Array|Get(acopy) _outactors_4)))

(event EventLaunchTransition
  ;[1 1 1] LaunchTransition
  (if (not (Utilities|Time|IsTimerActivebyHandle (Variables|Default|GetTimer)))
    (if (Class|KismetSystemLibrary|IsTimerPausedHandle (Variables|Default|GetTimer))
      (Utilities|Time|UnpauseTimerbyHandle (Variables|Default|GetTimer))
      (else
        (bind _returnvalue (Utilities|Time|SetTimerbyEvent (delegate Custom|UpdateTransition) (/ 1.0 (Variables|Transition|GetTransitionSpeed)) true))
        (Variables|Default|SetTimer _returnvalue)))
    (CallFunction|StartVFX)))

(fn ConstructionScript
  (Rendering|Material|SetVectorParameterValue "/Game/MaterialParametersCollection/TransitionParameters.TransitionParameters" "Center" (Math|Conversions|ToLinearColor(Vector) (Transformation|GetActorLocation)) :!class /Script/Engine.KismetMaterialLibrary))

(fn StartVFX
  ;[1 1 1] StartVFX
  (bind _returnvalue (Rendering|Material|GetScalarParameterValue "/Game/MaterialParametersCollection/TransitionParameters.TransitionParameters" "isNight" :!class /Script/Engine.KismetMaterialLibrary))
  (Rendering|SetVisibility (select (Math|Float|NearlyEqual(Float) _returnvalue -1.0 1e-06) (Variables|Default|GetWall_Dark) (Variables|Default|GetWall_Light)) true true)
  (Components|Activation|Activate (Variables|Default|GetPS_NightWorldGround) false)
  (Rendering|Material|SetScalarParameterValue "/Game/MaterialParametersCollection/TransitionParameters.TransitionParameters" "isTransitioning" 1.0 :!class /Script/Engine.KismetMaterialLibrary)
  (for _array_element (Variables|Default|GetWindManagerList)
    (Default|SetIsNight _array_element (Math|Float|NearlyEqual(Float) _returnvalue -1.0 1e-06))
    (CallFunction|UpdateSkySphere)))

(fn EndVFX
  ;[1 1 1] EndVFX
  (bind _returnvalue (Rendering|Material|GetScalarParameterValue "/Game/MaterialParametersCollection/TransitionParameters.TransitionParameters" "isNight" :!class /Script/Engine.KismetMaterialLibrary))
  (Rendering|SetVisibility (select (Math|Float|NearlyEqual(Float) _returnvalue 1.0 1e-06) (Variables|Default|GetWall_Dark) (Variables|Default|GetWall_Light)) false true)
  (Components|Activation|Deactivate (select (Math|Float|NearlyEqual(Float) _returnvalue 1.0 1e-06) (Variables|Default|GetPS_DayWorldGround) (Variables|Default|GetPS_NightWorldGround)))
  (Rendering|Material|SetScalarParameterValue "/Game/MaterialParametersCollection/TransitionParameters.TransitionParameters" "isTransitioning" 0.0 :!class /Script/Engine.KismetMaterialLibrary)
  (for _array_element (Variables|Default|GetWindManagerList)
    (Default|SetIsNight _array_element (Math|Float|NearlyEqual(Float) _returnvalue 1.0 1e-06))
    (Default|SetNightRatio (Variables|Default|GetSkySphere) (Math|Float|Clamp(Float) _returnvalue))))

(fn SwapVFX
  ;[1 1 1] SwapVFX
  (bind _returnvalue (Rendering|Material|GetScalarParameterValue "/Game/MaterialParametersCollection/TransitionParameters.TransitionParameters" "isNight" :!class /Script/Engine.KismetMaterialLibrary))
  (Rendering|SetVisibility (Variables|Default|GetWall_Dark) (not (Math|Float|NearlyEqual(Float) _returnvalue 1.0 1e-06)) true)
  (Rendering|SetVisibility (Variables|Default|GetWall_Light) (Math|Float|NearlyEqual(Float) _returnvalue 1.0 1e-06) true)
  (bind _returnvalue_2 (Rendering|Material|GetScalarParameterValue "/Game/MaterialParametersCollection/TransitionParameters.TransitionParameters" "isNight" :!class /Script/Engine.KismetMaterialLibrary))
  (Default|SetNightRatio (Variables|Default|GetSkySphere) (Math|Float|Clamp(Float) _returnvalue_2))
  (for _array_element (Variables|Default|GetWindManagerList)
    (Default|SetIsNight _array_element (Math|Float|NearlyEqual(Float) _returnvalue 1.0 1e-06))))

(fn UpdateGyroide
  (bind _gyroide (Variables|Gyroide|GetGyroide))
  (bind _gyroide_2 (Variables|Gyroide|GetGyroide))
  ;[1 1 1] UpdateGyroide
  (if (Utilities|IsValid _gyroide)
    (bind _returnvalue (Rendering|Material|GetScalarParameterValue "/Game/MaterialParametersCollection/TransitionParameters.TransitionParameters" "isTransitioning" :!class /Script/Engine.KismetMaterialLibrary))
    (if (or (>= (Variables|Transition|GetRadius) (Math|Vector|VectorLength (- (.Location (Math|Transform|BreakTransform (Transformation|GetWorldTransform (Variables|/Game/Blueprints/Gyroide/Horror_Gyroide_BP.Horror_Gyroide_BP_C|GetBody _gyroide)))) (.Location (Math|Transform|BreakTransform (Transformation|GetActorTransform)))))) (Math|Float|NearlyEqual(Float) _returnvalue 0.0 1e-06))
      (bind _returnvalue_2 (Rendering|Material|GetScalarParameterValue "/Game/MaterialParametersCollection/TransitionParameters.TransitionParameters" "isNight" :!class /Script/Engine.KismetMaterialLibrary))
      (Variables|/Game/Blueprints/ShinyEye/BP_ShinyEye_Final.BP_ShinyEye_Final_C|SetEyeSize _gyroide_2 (Math|Float|SelectFloat 3.0 0.0 (not (Math|Float|NearlyEqual(Float) _returnvalue_2 1.0 1e-06))))
      (Actor|Tick|SetActorTickEnabled _gyroide_2 (not (Math|Float|NearlyEqual(Float) _returnvalue_2 1.0 1e-06)))
      (Default|UpdateMaterial _gyroide_2)
      (if (not (not (Math|Float|NearlyEqual(Float) _returnvalue_2 1.0 1e-06)))
        (Transformation|SetActorTransform _gyroide_2 (Variables|Gyroide|GetInitialTransform))))))

(fn UpdateSkySphere
  ;[1 1 1] UpdateSkySphere
  (bind _returnvalue (Rendering|Material|GetScalarParameterValue "/Game/MaterialParametersCollection/TransitionParameters.TransitionParameters" "isNight" :!class /Script/Engine.KismetMaterialLibrary))
  (Default|SetNightRatio (Variables|Default|GetSkySphere) (|((Clamp(isNight,0,1))-(isNight*(1/({4B11FA53-45B9-36D0-1544-B5B176413343}/{85752165-499E-647A-C638-FA9D543570B5})))) _returnvalue)))